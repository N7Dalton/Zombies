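; Game mode that runs wave-based zombie spawning, starting the first wave on BeginPlay.
; Each wave's zombie count scales with the wave number, split between two spawn transforms.
; ZombiesKilled decrements the remaining count and, at zero, advances the wave until MaxWaves is reached.
; Each new wave shows wave UI through the first-person character, then spawns zombies after a short delay.
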(event Custom|StartGame
  ;[1 1 1] start game
  (CallFunction|SpawnZombies))

(event Custom|SpawnZombies
  (bind _output_get (Variables|Default|SetzombieTotal (* (Variables|Default|GetCurrentWave) 4)))
  (Variables|Default|SetZombies%20Left _output_get)
  (bind _index (Utilities|FlowControl|ForLoopwithBreak 0 _output_get :!label _label)
    (:LoopBody
      (if (== _index (/ (Variables|Default|GetzombieTotal) 2))
        (goto _label Break)
        (else
          (Game|SpawnActorfromClass "/Game/_Main/Zombro/BP_Zombie.BP_Zombie_C" (Variables|Default|GetSpawnLoco1) "Undefined" "MultiplyWithRoot" 0 0))))
    (:Completed
      (Utilities|FlowControl|ForLoopwithBreak 1 (/ (Variables|Default|GetzombieTotal) 2)
        (:LoopBody
          (Game|SpawnActorfromClass "/Game/_Main/Zombro/BP_Zombie.BP_Zombie_C" (Variables|Default|GetspawnLoco2) "Undefined" "MultiplyWithRoot" 0 0))))))

(event Custom|ZombiesKilled
  (bind _result (Math|Integer|DecrementInt (Variables|Default|GetZombies%20Left))
    (:%20%20
      (if (== _result 0)
        (CallFunction|WaveIncrement)
        (Development|PrintText "Wavenext")))))

(event Custom|WaveIncrement
  (if (not (== (Variables|Default|GetCurrentWave) (Variables|Default|GetMaxWaves)))
    (Math|Integer|IncrementInt (Variables|Default|GetCurrentWave)
      (:%20%20
        (CallFunction|WaveStart)))))

(event Custom|WaveStart
  ;[1 1 1] start next wave
  (bind _asbp_first_person_character (Utilities|Casting|CastToBP_FirstPersonCharacter (Game|GetPlayerCharacter 0)))
  (Default|ShowWaveUI _asbp_first_person_character (Variables|Default|GetCurrentWave))
  (Utilities|FlowControl|Delay 5.0)
  (CallFunction|SpawnZombies))

(event EventBeginPlay
  ;[1 1 1] start game
  (CallFunction|StartGame))

(event EventTick
  (params (DeltaSeconds :type Float%20%28single-precision%29)))

(fn ConstructionScript)