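; Zombie enemy that chases the player from spawn, attacks in melee and dies from point damage.
; A looping AI MoveTo targets the player controller, and PawnSensing sets run speed on sighting the player.
; An attack montage notify triggers a sphere overlap at the arrow component to damage the player.
; Hits play reactions; death disables capsule collision, reports the kill to ZombieGamemode, then destroys the actor after a delay.
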(event OnSeePawn(PawnSensing)
  (params (Pawn :type Pawn%20Object%20Reference))
  ;[1 1 1] Start running when near player
  (Variables|/Script/Engine.CharacterMovementComponent|SetMaxWalkSpeed (Variables|Character|GetCharacterMovement) 3.6e+02))

(event Custom|RunToPlayer
  ;[1 1 1] Run to player
  (if (not (Variables|Default|GetIsDead))
    (AI|AIMoveTo self "0, 0, 0" (Game|GetPlayerController 0) 4e+01 false
      (:OnSuccess
        (CallFunction|AttackPlayer))
      (:OnFail
        (CallFunction|RuntoPlayer)))))

(event Custom|AttackPlayer
  ;[1 1 1] if close enough attack player
  (Animation|Montage|PlayMontage (Variables|Character|GetMesh) "/Game/_Main/Zombro/Animations/zombie_attack_Montage1.zombie_attack_Montage1"
    (:OnCompleted
      (CallFunction|RuntoPlayer))
    (:OnNotifyBegin
      (bind (_outactors _returnvalue) (Collision|SphereOverlapActors (Transformation|GetWorldLocation (Variables|Default|GetArrow1)) 75.0 (Utilities|Array|MakeArray "ObjectTypeQuery3") "/Game/_Main/Blueprints/BP_FirstPersonCharacter.BP_FirstPersonCharacter_C" (Utilities|Array|MakeArray self)))
      (if _returnvalue
        (for _array_element _outactors
          (Game|Damage|ApplyDamage _array_element 2e+01 (Pawn|GetController) self "/Script/Engine.DamageType"))))))

(event Custom|Death
  ;[1 1 1] On Death function
  (Variables|Default|SetIsDead true)
  (Components|Movement|StopMovementImmediately (Variables|Character|GetCharacterMovement))
  (Animation|Montage|PlayMontage (Variables|Character|GetMesh) "/Game/_Main/Zombro/Animations/zombie_death_Montage.zombie_death_Montage"
    (:then
      ;[1 1 1] turn off capsule collider
      (Collision|SetCollisionResponsetoChannel (Variables|Collision|GetCapsuleComponent) "ECC_Pawn" "ECR_Overlap")
      (Collision|SetCollisionEnabled (Variables|Collision|GetCapsuleComponent) "NoCollision")
      (bind _aszombie_gamemode (Utilities|Casting|CastToZombieGamemode (Game|GetGameMode)))
      (Default|ZombiesKilled _aszombie_gamemode)
      (Utilities|FlowControl|Delay 1e+01)
      (Actor|DestroyActor))))

(event EventBeginPlay
  ;[1 1 1] Basically void start
  (CallFunction|RuntoPlayer))

(event Game|Damage|EventPointDamage
  (params (Damage :type Float%20%28single-precision%29) (DamageType :type Damage%20Type%20Object%20Reference) (HitLocation :type Vector :default "0, 0, 0") (HitNormal :type Vector :default "0, 0, 0") (HitComponent :type Primitive%20Component%20Object%20Reference) (BoneName :type Name :default "None") (ShotFromDirection :type Vector :default "0, 0, 0") (InstigatedBy :type Controller%20Object%20Reference) (DamageCauser :type Actor%20Object%20Reference) (HitInfo :type Hit%20Result%20Structure%20%28by%20ref%29))
  ;[1 1 1] Apply damage to zombie
  (if (not (Variables|Default|GetIsDead))
    (if (<= (Variables|Default|Gethealth) 0.0)
      (CallFunction|Death)
      (else
        (bind _output_get (Variables|Default|Sethealth (- (Variables|Default|Gethealth) Damage)))
        (Development|PrintString (Utilities|String|ToString(Float) _output_get))
        (if (<= _output_get 0.0)
          (CallFunction|Death)
          (else
            (Animation|Montage|PlayMontage (Variables|Character|GetMesh) "/Game/_Main/Zombro/Animations/Zombie_Reaction_Hit_mixamo_com_Montage.Zombie_Reaction_Hit_mixamo_com_Montage")))))))

(fn ConstructionScript)